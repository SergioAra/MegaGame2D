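; Player character Blueprint that handles the sprite's visual feedback for damage, invincibility, charge levels and 2D mode switching.
; Damage, full-charge and partial-charge events each play a timeline that feeds FlashSprite, which sets flash color and scaled intensity on a dynamic material instance.
; Invincibility toggles sprite visibility on a looping timer until it ends and restores visibility.
; Switching 2D mode swaps the sprite between unlit and lit materials.
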(event `OnSwitch2D`
  (params (bIs2DEnabled :type Boolean))
  (`PrimitiveComponent.SetMaterial` (`self.Sprite`) 0 (select `bool` bIs2DEnabled :`false` "/Game/Materials/Sprite/MI_CustomLitSpriteMaterial.MI_CustomLitSpriteMaterial" :`true` "/Game/Materials/Sprite/MI_CustomUnlitSpriteMaterial.MI_CustomUnlitSpriteMaterial" :!type "MaterialInterface Object Reference")))

(event `self.OnDamageVFX`
  (`TimelineComponent.SetPlayRate` (`self.FlashVFX`) (`self.DamageVFXPlayRate`))
  (bind (_direction _multiplier _color) (`Timeline|FlashVFX` :!via `PlayFromStart`)
    (:`Update`
      (`self.FlashSprite` _multiplier _color (`self.DamageVFXScale`)))))

(event `self.OnInvincibilityVFX`
  (bind _returnvalue (`KismetSystemLibrary.K2_SetTimerDelegate` (delegate `FlickerSprite`) (`self.InvincibilityFlickerInterval`) true true))
  (set `self.FlickerHandle` _returnvalue))

(event `FlickerSprite`
  (bind _sprite (`self.Sprite`))
  (`SceneComponent.SetVisibility` _sprite (not (`SceneComponent.bVisible` _sprite)) true))

(event `self.OnEndInvincibility`
  (`SceneComponent.SetVisibility` (`self.Sprite`) true true)
  (`KismetSystemLibrary.K2_ClearAndInvalidateTimerHandle` (`self.FlickerHandle`)))

(event `self.OnFlashFullCharge`
  (`TimelineComponent.SetPlayRate` (`self.FlashFullCharge`) (`self.FullChargeVFXPlayRate`))
  (bind (_direction _multiplier _color) (`Timeline|FlashFullCharge` :!via `PlayFromStart`)
    (:`Update`
      (`self.FlashSprite` _multiplier _color (`self.FullChargeVFXScale`)))))

(event `self.OnFlashPartialCharge`
  (`TimelineComponent.SetPlayRate` (`self.FlashPartialCharge`) (`self.PartialChargeVFXPlayRate`))
  (bind (_direction _multiplier _color) (`Timeline|FlashPartialCharge` :!via `PlayFromStart`)
    (:`Update`
      (`self.FlashSprite` _multiplier _color (`self.PartialChargeVFXScale`)))))

(fn `FlashSprite`
  (params (Alpha :type "Float (double-precision)") (Color :type "LinearColor Structure") (Scale :type "Float (double-precision)"))
  (bind _dynamicmaterialinstance (`self.DynamicMaterialInstance`))
  (`MaterialInstanceDynamic.SetScalarParameterValue` _dynamicmaterialinstance "FlashMultiplier" (* Alpha Scale))
  (`MaterialInstanceDynamic.SetVectorParameterValue` _dynamicmaterialinstance "FlashColor" Color))

(fn `UserConstructionScript`
  (`parent.UserConstructionScript`))