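; Base Blueprint for sprite-based enemy characters, handling their visual response to 2D mode switches and damage.
; OnSwitch2D swaps the sprite material between custom unlit for 2D and custom lit otherwise.
; OnDamageVFX restarts the FlashVFX timeline at a configurable rate, driving flash color and scaled multiplier parameters on a dynamic material instance.
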(event `OnSwitch2D`
  (params (bIs2DEnabled :type Boolean))
  (`PrimitiveComponent.SetMaterial` (`self.Sprite`) 0 (select `bool` bIs2DEnabled :`false` "/Game/Materials/Sprite/MI_CustomLitSpriteMaterial.MI_CustomLitSpriteMaterial" :`true` "/Game/Materials/Sprite/MI_CustomUnlitSpriteMaterial.MI_CustomUnlitSpriteMaterial" :!type "MaterialInterface Object Reference")))

(event `self.OnDamageVFX`
  (bind _dynamicmaterialinstance (`self.DynamicMaterialInstance`))
  (`TimelineComponent.SetPlayRate` (`self.FlashVFX`) (`self.DamageVFXPlayRate`))
  (bind (_direction _multiplier _color) (`Timeline|FlashVFX` :!via `PlayFromStart`)
    (:`Update`
      (`MaterialInstanceDynamic.SetScalarParameterValue` _dynamicmaterialinstance "FlashMultiplier" (* _multiplier (`self.DamageVFXScale`)))
      (`MaterialInstanceDynamic.SetVectorParameterValue` _dynamicmaterialinstance "FlashColor" _color))))

(fn `UserConstructionScript`)